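; BP_portal01 is a portal actor in the endless staircase system that moves the player to a linked portal.
; When the player character overlaps its Collision component and OtherPortal is valid, the player's location is set to the same world-space offset from the other portal.
; Only position changes, without sweep or rotation adjustment, so matching portal surroundings would make the jump read as continuous.
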(event `self.collision.OnComponentBeginOverlap`
  (params (OverlappedComponent :type "PrimitiveComponent Object Reference") (OtherActor :type "Actor Object Reference") (OtherComp :type "PrimitiveComponent Object Reference") (OtherBodyIndex :type Integer) (bFromSweep :type Boolean) (SweepResult :type "HitResult Structure (by ref)"))
  (bind _returnvalue (`GameplayStatics.GetPlayerCharacter` 0))
  (bind _otherportal (`self.OtherPortal`))
  (if (== OtherActor _returnvalue)
    (`/Engine/EditorBlueprintResources/StandardMacros.IsValid` _otherportal
      (:`Is Valid`
        (`self.K2_SetActorLocation` _returnvalue (+ (- (`self.K2_GetActorLocation` _returnvalue) (`self.K2_GetActorLocation`)) (`self.K2_GetActorLocation` _otherportal)) false false)))))

(fn `UserConstructionScript`)